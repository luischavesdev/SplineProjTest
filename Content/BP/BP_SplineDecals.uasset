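; BP_SplineDecals is an actor that lays a row of decals along a spline at runtime.
; BeginPlay starts a looping timer that destroys and respawns every decal component on each tick.
; Decals are spaced by DecalSize along the spline length, share one material and scale, and take only yaw from the spline.
; A similar placement chain in the construction script is disconnected, so construction does nothing.
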(event `self.ReceiveBeginPlay`
  (bind _returnvalue (`KismetSystemLibrary.K2_SetTimerDelegate` (delegate `CustomTick`) (`self.TimerInterval`) true))
  (set `self.TimerRef` _returnvalue))

(event `CustomTick`
  (bind _spline (`self.Spline`))
  (bind _decalcomponents (`self.DecalComponents`))
  (for _array_element _decalcomponents
    (`ActorComponent.K2_DestroyComponent` _array_element))
  (`KismetArrayLibrary.Array_Clear` _decalcomponents)
  (bind _output_get (set `self.SplineDivisions` (`KismetMathLibrary.FTrunc` (/ (`SplineComponent.GetSplineLength` (`self.Spline`)) (`self.DecalSize`)))))
  (for _index (range (+ _output_get 1))
    (bind _returnvalue (`AddComponent|NODE_AddDecalComponent-1` :`RelativeTransform` (`KismetMathLibrary.MakeTransform` (0.0 0.0 0.0) (struct) (`self.DecalScale`))))
    (`DecalComponent.SetDecalMaterial` _returnvalue (`self.DecalRef`))
    (bind _returnvalue_2 (* _index (`self.DecalSize`)))
    (bind (_returnvalue_roll _returnvalue_pitch _returnvalue_yaw) (`KismetMathLibrary.BreakRotator` (`SplineComponent.GetRotationAtDistanceAlongSpline` _spline _returnvalue_2 "World")))
    (`SceneComponent.K2_SetWorldLocationAndRotation` _returnvalue (`SplineComponent.GetLocationAtDistanceAlongSpline` _spline _returnvalue_2 "World") (`KismetMathLibrary.MakeRotator` 0.0 0.0 _returnvalue_yaw) false false)
    (`KismetArrayLibrary.Array_Add` (`self.DecalComponents`) _returnvalue)))

(fn `UserConstructionScript`)