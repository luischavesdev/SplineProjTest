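; BP_SplineTest is a test actor that builds spline meshes along a spline and along a copy projected onto surrounding geometry.
; The construction script tiles MeshRef along Spline at mesh-bound intervals, clamping tangents to that length.
; It line-traces along the spline's default up vector at finer ProjectionResolution steps, rebuilding DeformedSpline from the hits.
; A second row of spline meshes then links each pair of projected points.
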(fn `CalculateSplineMeshStartEnd`
  (params (Index :type Integer) (IsStart :type Boolean))
  (returns (Position :type "Vector Structure") (Tangent :type "Vector Structure"))
  (bind _spline (`self.Spline`))
  (bind _returnvalue (* (`KismetMathLibrary.SelectInt` Index (+ Index 1) IsStart) (`self.MeshLength`)))
  (return (`SplineComponent.GetLocationAtDistanceAlongSpline` _spline _returnvalue "Local") (`KismetMathLibrary.ClampVectorSize` (`SplineComponent.GetTangentAtDistanceAlongSpline` _spline _returnvalue "Local") 0.0 (`self.MeshLength`))))

(fn `UserConstructionScript`
  (bind _deformedspline (`self.DeformedSpline`))
  (bind _meshlength (`self.MeshLength`))
  (`SplineComponent.ClearSplinePoints` (`self.DeformedSpline`) true)
  (bind _output_get (set `self.MeshLength` (.x (`.BoxExtent` (`KismetMathLibrary.BreakBoxSphereBounds` (`StaticMesh.GetBounds` (`self.MeshRef`)))))))
  (set `self.SplineDivisions` (`KismetMathLibrary.FTrunc` (/ (`SplineComponent.GetSplineLength` (`self.Spline`)) _output_get)))
  (bind _output_get_2 (set `self.ResolutionLength` (/ (`self.MeshLength`) (`self.ProjectionResolution`))))
  (bind _output_get_3 (set `self.ResolutionDivisions` (`KismetMathLibrary.FTrunc` (/ (`SplineComponent.GetSplineLength` (`self.Spline`)) _output_get_2))))
  (for _index (range (+ (`self.SplineDivisions`) 1))
    (bind _returnvalue (`AddComponent|NODE_AddSplineMeshComponent-0`))
    (`StaticMeshComponent.SetStaticMesh` _returnvalue (`self.MeshRef`))
    (`SplineMeshComponent.SetForwardAxis` _returnvalue "X" true)
    (bind (_position _tangent) (`self.CalculateSplineMeshStartEnd` _index true))
    (bind (_position_2 _tangent_2) (`self.CalculateSplineMeshStartEnd` _index))
    (`SplineMeshComponent.SetStartAndEnd` _returnvalue _position _tangent _position_2 _tangent_2 true))
  (for _index_2 (range (+ _output_get_3 1))
    (bind _returnvalue_2 (`SplineComponent.GetLocationAtDistanceAlongSpline` (`self.Spline`) (* _index_2 (`self.ResolutionLength`)) "World"))
    (bind _outhit (`KismetSystemLibrary.LineTraceSingle` :`Start` _returnvalue_2 :`End` (+ _returnvalue_2 (* (`SplineComponent.GetDefaultUpVector` (`self.Spline`) "World") (`self.CastDistance`))) :`TraceChannel` "TraceTypeQuery1" :`DrawDebugType` "ForDuration" :`DrawTime` 1.0))
    (bind (_bblockinghit _binitialoverlap _time _distance _location) (`GameplayStatics.BreakHitResult` _outhit))
    (if _bblockinghit
      (`SplineComponent.AddSplinePoint` (`self.DeformedSpline`) _location "World" true)))
  (for _index_3 (range (+ (- (`SplineComponent.GetNumberOfSplinePoints` (`self.DeformedSpline`)) 2) 1))
    (bind _returnvalue_3 (`AddComponent|NODE_AddSplineMeshComponent-1`))
    (`StaticMeshComponent.SetStaticMesh` _returnvalue_3 (`self.MeshRef`))
    (`SplineMeshComponent.SetForwardAxis` _returnvalue_3 "X" true)
    (bind (_location_2 _tangent_3) (`SplineComponent.GetLocationAndTangentAtSplinePoint` _deformedspline _index_3 "Local"))
    (bind (_location_3 _tangent_4) (`SplineComponent.GetLocationAndTangentAtSplinePoint` _deformedspline (+ _index_3 1) "Local"))
    (`SplineMeshComponent.SetStartAndEnd` _returnvalue_3 _location_2 (`KismetMathLibrary.ClampVectorSize` _tangent_3 0.0 _meshlength) _location_3 (`KismetMathLibrary.ClampVectorSize` _tangent_4 0.0 _meshlength) true)))