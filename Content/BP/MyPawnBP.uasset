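; Player pawn for a tile puzzle where queued move and turn commands drive a cube, with drag-to-orbit and zoom camera.
; Buttons fill a capped action queue; OK executes it sequentially through looping-timer interpolation, each completed step triggering the next.
; Overlap sensors find neighboring tiles for movement and rotation targets, rejecting edge moves.
; The tile below triggers a hazard reset or winning-tile check, and detection first runs on the GameMode's tiles-spawned event.
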(event `InputAxis|TurnCamera`
  (params (AxisValue :type "Float (single-precision)"))
  ;[1 1 1] Camera
  (if (`self.CameraIsPressed`)
    (`self.AddControllerYawInput` (* AxisValue (`self.CameraMovMultiplier`)))))

(event `InputAction|CameraInput`
  (params (Key :type "Key Structure"))
  (bind _returnvalue (`GameplayStatics.GetPlayerController` 0))
  ;[1 1 1] Camera
  (:`Pressed`
    (set `self.CameraIsPressed` true)
    (set `PlayerController.bShowMouseCursor` false _returnvalue))
  (:`Released`
    (set `self.CameraIsPressed` false)
    (set `PlayerController.bShowMouseCursor` true _returnvalue)))

(event `ResetToStartTile`
  (bind _cube (`self.Cube`))
  ;[1 1 1] ResetToStart
  (`SceneComponent.K2_SetWorldLocation` _cube (`self.InitialLocation`) false false)
  (`SceneComponent.K2_SetRelativeRotation` _cube (`self.InitialRotation`) false false)
  (set `self.IsActing` false)
  (`KismetArrayLibrary.Array_Clear` (`self.ActionsQueue`))
  (`self.Detect Adjacent`))

(event `InputAxis|ZoomCamera`
  (params (AxisValue :type "Float (single-precision)"))
  (bind _springarm (`self.SpringArm`))
  ;[1 1 1] Camera
  (set `SpringArmComponent.TargetArmLength` (`KismetMathLibrary.FClamp` (+ (* AxisValue (`self.CameraZoomMultiplier`)) (`SpringArmComponent.TargetArmLength` _springarm)) (`self.MinCamZoom`) (`self.MaxCamZoom`)) _springarm))

(event `self.ReceiveBeginPlay`
  (bind _returnvalue (`GameplayStatics.GetPlayerCameraManager` 0))
  (bind _cube (`self.Cube`))
  ;[1 1 1] BeginPlay
  (set `self.InitialLocation` (`SceneComponent.K2_GetComponentLocation` _cube))
  (set `self.InitialRotation` (`SceneComponent.RelativeRotation` _cube))
  (set `PlayerController.bShowMouseCursor` true (`GameplayStatics.GetPlayerController` 0))
  (set `PlayerCameraManager.ViewPitchMin` -90.0 _returnvalue)
  (set `PlayerCameraManager.ViewPitchMax` -5.0 _returnvalue)
  (set `self.Sensors` (`|MakeArray` (`self.SensorFront`) (`self.SensorRight`) (`self.SensorLeft`) (`self.SensorBack`)))
  (bind _asmy_game_mode (cast `/Game/BP/MyGameMode` (`GameplayStatics.GetGameMode`))
    (:`then`
      (bind _output_get (set `self.MyGameModeRef` _asmy_game_mode))
      (add `/Game/BP/MyGameMode.AllTilesSpawned` _output_get (delegate `CallDetectAdjacent`)))
    (:`CastFailed`
      (`KismetSystemLibrary.PrintString` "BadCast" true true (struct :`R` 1.0 :`B` 0.207142 :`A` 1.0)))))

(event `InputAxis|LookUpCamera`
  (params (AxisValue :type "Float (single-precision)"))
  ;[1 1 1] Camera
  (if (`self.CameraIsPressed`)
    (`self.AddControllerPitchInput` (* (`self.CameraMovMultiplier`) AxisValue))))

(event `CallDetectAdjacent`
  ;[1 1 1] BeginPlay
  (`self.Detect Adjacent`))

(event `UpButton`
  (bind _actionsqueue (`self.ActionsQueue`))
  (bind _returnvalue (`KismetArrayLibrary.Array_Length` _actionsqueue))
  ;[1 1 1] Inputs
  (if (not (`self.IsActing`))
    (`KismetSystemLibrary.PrintString` "Up")
    (set `self.Action` 0)
    (if (< _returnvalue (`self.MaxAction`)) :!label _label
      (`KismetArrayLibrary.Array_Set` _actionsqueue _returnvalue (stale `LeftButton` _output_get) true)
      (else
        (`KismetSystemLibrary.PrintString` "Max Moves Reached" true true (struct :`R` 1.0 :`B` 0.142498 :`A` 1.0))))))

(event `RotateInput`
  (params (Clockwise :type Boolean))
  ;[1 1 1] Rotate
  (if (`self.CanRotate`)
    (set `self.CanRotate` false)
    (bind _targetrotation (`self.GetTargetRotation` Clockwise))
    (set `self.TargetRotation` _targetrotation)
    (bind _returnvalue (`KismetSystemLibrary.K2_SetTimerDelegate` (delegate `Rotate`) 0.01 true))
    (set `self.RotateHandle` _returnvalue)))

(event `RightButton`
  ;[1 1 1] Inputs
  (if (not (`self.IsActing`))
    (`KismetSystemLibrary.PrintString` "Right")
    (set `self.Action` 1)
    (goto _label)))

(event `MoveInput`
  (params (Forwards :type Boolean))
  ;[1 1 1] Movement
  (if (`self.CanMove`)
    (if (`/Game/BP/TileBP.IsEdge` (`|GetArrayItem` (`self.AdjacentTiles`) (`KismetMathLibrary.SelectInt` 0 3 Forwards)))
      (`KismetSystemLibrary.PrintString` "Invalid Move" true true (struct :`R` 1.0 :`B` 0.142498 :`A` 1.0))
      (`KismetArrayLibrary.Array_Clear` (`self.ActionsQueue`))
      (set `self.IsActing` false)
      (else
        (set `self.CanMove` false)
        (bind _returnvalue (`KismetSystemLibrary.K2_SetTimerDelegate` (delegate `MoveTo`) 0.01 true))
        (set `self.MoveHandle` _returnvalue)))))

(event `LeftButton`
  ;[1 1 1] Inputs
  (if (not (`self.IsActing`))
    (`KismetSystemLibrary.PrintString` "Left")
    (bind _output_get (set `self.Action` 2))
    (goto _label)))

(event `Rotate`
  (bind _cube (`self.Cube`))
  (bind (_targetrotation_roll _targetrotation_pitch _targetrotation_yaw) (`KismetMathLibrary.BreakRotator` (`self.TargetRotation`)))
  (bind (_relativerotation_roll _relativerotation_pitch) (`KismetMathLibrary.BreakRotator` (`SceneComponent.RelativeRotation` _cube)))
  (bind (_returnvalue_roll _returnvalue_pitch _returnvalue_yaw) (`KismetMathLibrary.BreakRotator` (`KismetMathLibrary.RInterpTo` (`SceneComponent.RelativeRotation` _cube) (`self.TargetRotation`) (`GameplayStatics.GetWorldDeltaSeconds`) (`self.RotationSpeed`))))
  ;[1 1 1] Rotate
  (`SceneComponent.K2_SetRelativeRotation` _cube (`KismetMathLibrary.MakeRotator` _relativerotation_roll _relativerotation_pitch _returnvalue_yaw) false false)
  (if (`KismetMathLibrary.NearlyEqual_FloatFloat` (`KismetMathLibrary.Abs` _returnvalue_yaw) (`KismetMathLibrary.Abs` _targetrotation_yaw) 0.1)
    (`self.Detect Adjacent`)
    (set `self.CanRotate` true)
    (`KismetSystemLibrary.K2_ClearAndInvalidateTimerHandle` (`self.RotateHandle`))
    (`self.Check Next Action`)))

(event `DownButton`
  ;[1 1 1] Inputs
  (if (not (`self.IsActing`))
    (`KismetSystemLibrary.PrintString` "Down")
    (set `self.Action` 3)
    (goto _label)))

(event `MoveTo`
  (bind (_returnvalue_x _returnvalue_y _returnvalue_z) (`KismetMathLibrary.BreakVector` (`SceneComponent.K2_GetComponentLocation` (`self.Cube`))))
  ;[1 1 1] Movement
  (bind (_returnvalue_x_2 _returnvalue_y_2 _returnvalue_z_2) (`KismetMathLibrary.BreakVector` (`self.K2_GetActorLocation` (`|GetArrayItem` (`self.AdjacentTiles`) (`KismetMathLibrary.SelectInt` 0 3 (stale `MoveInput` Forwards))))))
  (bind (_returnvalue_x_3 _returnvalue_y_3) (`KismetMathLibrary.BreakVector` (`KismetMathLibrary.VInterpTo` (`KismetMathLibrary.MakeVector` _returnvalue_x _returnvalue_y _returnvalue_z) (`KismetMathLibrary.MakeVector` _returnvalue_x_2 _returnvalue_y_2 _returnvalue_z_2) (`GameplayStatics.GetWorldDeltaSeconds`) (`self.MoveSpeed`))))
  (`SceneComponent.K2_SetWorldLocation` (`self.Cube`) (`KismetMathLibrary.MakeVector` _returnvalue_x_3 _returnvalue_y_3 _returnvalue_z) false false)
  (if (== (`KismetMathLibrary.MakeVector2D` _returnvalue_x_3 _returnvalue_y_3) (`KismetMathLibrary.MakeVector2D` _returnvalue_x_2 _returnvalue_y_2) :`ErrorTolerance` 0.1)
    (set `self.CanMove` true)
    (`KismetSystemLibrary.K2_ClearAndInvalidateTimerHandle` (`self.MoveHandle`))
    (`self.Detect Adjacent`)
    (`self.Check Next Action`)))

(event `OkButton`
  ;[1 1 1] Inputs
  (`KismetSystemLibrary.PrintString` "Enter")
  (set `self.IsActing` true)
  (`self.Check Next Action`))

(event `TrashButton`
  ;[1 1 1] Inputs
  (`KismetSystemLibrary.PrintString` "Clear")
  (`KismetArrayLibrary.Array_Clear` (`self.ActionsQueue`)))

(fn `Check Next Action`
  (bind _actionsqueue (`self.ActionsQueue`))
  (bind _actionsqueue_2 (`self.ActionsQueue`))
  (if (`KismetArrayLibrary.Array_IsEmpty` _actionsqueue)
    (set `self.IsActing` false)
    (return)
    (else
      (switch `int` (`|GetArrayItem` _actionsqueue)
        (:`0`
          (`|ExecutionSequence`
            (:`then_0`
              (`KismetArrayLibrary.Array_Remove` _actionsqueue_2 :!label _label)
              (`KismetSystemLibrary.PrintString` (`KismetStringLibrary.Conv_IntToString` (`KismetArrayLibrary.Array_Length` _actionsqueue_2))))
            (:`then_1`
              (`self.MoveInput` true))))
        (:`1`
          (`|ExecutionSequence`
            (:`then_0`
              (goto _label))
            (:`then_1`
              (`self.RotateInput` true))))
        (:`2`
          (`|ExecutionSequence`
            (:`then_0`
              (goto _label))
            (:`then_1`
              (`self.RotateInput` false))))
        (:`3`
          (`|ExecutionSequence`
            (:`then_0`
              (goto _label))
            (:`then_1`
              (`self.MoveInput` false))))))))

(fn `Detect Adjacent`
  (bind _adjacenttiles (`self.AdjacentTiles`))
  (bind _winningtiles (`self.WinningTiles`))
  (bind _actionsqueue (`self.ActionsQueue`))
  (for (_array_element _array_index) (`self.Sensors`)
    (bind _astile_bp (cast `/Game/BP/TileBP` (`|GetArrayItem` (`PrimitiveComponent.GetOverlappingActors` _array_element "/Game/BP/TileBP.TileBP_C")))
      (:`then`
        (`KismetArrayLibrary.Array_Set` _adjacenttiles _array_index _astile_bp))
      (:`CastFailed`
        (`KismetArrayLibrary.Array_Set` _adjacenttiles _array_index))))
  (bind _astile_bp_2 (cast `/Game/BP/TileBP` (`|GetArrayItem` (`PrimitiveComponent.GetOverlappingActors` (`self.SensorBelow`) "/Game/BP/TileBP.TileBP_C")))
    (:`then`
      (if (`/Game/BP/TileBP.IsHazard` _astile_bp_2)
        (`self.ResetToStartTile`)
        (else
          (if (`KismetMathLibrary.Conv_IntToBool` (`KismetArrayLibrary.Array_Length` _winningtiles))
            (if (== (`/Game/BP/TileBP.TileNum` _astile_bp_2) (`|GetArrayItem` _winningtiles))
              (`KismetArrayLibrary.Array_Remove` _actionsqueue)
              (if (== (`KismetArrayLibrary.Array_Length` _actionsqueue) 0)
                (`KismetSystemLibrary.PrintString` "Congratulations!" true true (struct :`R` 0.228305 :`G` 1.0 :`A` 1.0)))))
          (return))))
    (:`CastFailed`
      (return))))

(fn `GetTargetRotation`
  (params (Clockwise :type Boolean))
  (returns (TargetRotation :type "Rotator Structure"))
  (return (`KismetMathLibrary.FindLookAtRotation` (`SceneComponent.K2_GetComponentLocation` (`self.Cube`)) (`self.K2_GetActorLocation` (`|GetArrayItem` (`self.AdjacentTiles`) (`KismetMathLibrary.SelectInt` 1 2 Clockwise))))))

(fn `UserConstructionScript`)