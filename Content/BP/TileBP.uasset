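; TileBP is a board tile that discovers its neighbors, with optional start and edge roles.
; On BeginPlay it creates tile and icon materials, registers with MyGameMode, then spawns and possesses MyPawnBP on the start tile or offsets the texture of edge tiles.
; When the game mode signals all tiles have spawned, four directional feelers use overlap checks to fill AdjacentTiles.
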(event `self.ReceiveBeginPlay`
  (set `self.Feelers` (`|MakeArray` (`self.FeelerFront`) (`self.FeelerRight`) (`self.FeelerLeft`) (`self.FeelerBack`)))
  (bind _returnvalue (`PrimitiveComponent.CreateDynamicMaterialInstance` (`self.TileMesh`) 0 "/Game/Tiles/TileMatInst.TileMatInst" "None"))
  (set `self.MatInstRef` _returnvalue)
  (bind _returnvalue_2 (`PrimitiveComponent.CreateDynamicMaterialInstance` (`self.IconMesh`) 0 "/Game/Tiles/TileIconMatInst.TileIconMatInst" "None"))
  (set `self.IconMatInstRef` _returnvalue_2)
  (bind _asmy_game_mode (cast `/Game/BP/MyGameMode` (`GameplayStatics.GetGameMode`))
    (:`then`
      (bind _output_get (set `self.MyGameModeRef` _asmy_game_mode))
      (add `/Game/BP/MyGameMode.AllTilesSpawned` _output_get (delegate `FeelAdjacent`))
      (`/Game/BP/MyGameMode.OnTileSpawn` _output_get)
      (`MaterialInstanceDynamic.SetTextureParameterValue` (`self.IconMatInstRef`) "IconTexture" (`self.IconTexture`))
      (`|ExecutionSequence`
        (:`then_0`
          (if (`self.IsStart`)
            (bind _returnvalue_3 (`|SpawnActorFromClass` "/Game/BP/MyPawnBP.MyPawnBP_C" (`self.GetTransform`) "Undefined" "MultiplyWithRoot" null self null))
            (`Controller.Possess` (`GameplayStatics.GetPlayerController` 0) _returnvalue_3)))
        (:`then_1`
          (if (`self.IsEdge`)
            (`MaterialInstanceDynamic.SetScalarParameterValue` (`self.MatInstRef`) "UOffset" 0.5)))))
    (:`CastFailed`
      (`KismetSystemLibrary.PrintString` "BadCast" true true (struct :`R` 1.0 :`B` 0.207142 :`A` 1.0)))))

(event `FeelAdjacent`
  ;[1 1 1] FeelAdjacentOnStart
  (for _array_element (`self.Feelers`)
    (bind _astile_bp (cast `/Game/BP/TileBP` (`|GetArrayItem` (`PrimitiveComponent.GetOverlappingActors` _array_element "TileBP_C"))))
    (`KismetArrayLibrary.Array_AddUnique` (`self.AdjacentTiles`) _astile_bp)))

(fn `UserConstructionScript`)