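; Spline actor that projects its shape as a colored decal by rendering spline meshes into a render target.
; Spline mesh segments are built along the spline at intervals derived from mesh bounds.
; A SceneCapture2D showing only this actor writes to an RG8 target sized from the decal, feeding its dynamic material.
; Setup runs at construction, capture and material again on BeginPlay, while CustomTick rebuilds meshes for play-mode editing.
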(event `self.ReceiveBeginPlay`
  (bind _showonlyactors (`self.ShowOnlyActors`))
  (`parent.ReceiveBeginPlay`)
  (`self.Setup Mat and RT`)
  (`KismetArrayLibrary.Array_Clear` _showonlyactors)
  (`KismetArrayLibrary.Array_Add` _showonlyactors self)
  (set `SceneCaptureComponent.ShowOnlyActors` _showonlyactors (`self.SceneCaptureComponent2D`)))

(event `self.CustomTick`
  (bind (_decalsize_x _decalsize_y _decalsize_z) (`KismetMathLibrary.BreakVector` (`DecalComponent.DecalSize` (`self.Decal`))))
  ;[1 1 1] Can be discarded if spline is only to be edited while in editor and not in play mode
  (`self.ClearMeshes`
    (:`ExecOut`
      (`self.Setup Mesh`)
      (set `SceneCaptureComponent2D.OrthoWidth` (* _decalsize_z 2.0) (`self.SceneCaptureComponent2D`)))))

(fn `CalculateSplineMeshStartEnd`
  (params (Index :type Integer) (IsStart :type Boolean))
  (returns (Position :type "Vector Structure") (Tangent :type "Vector Structure"))
  (bind _spline (`self.Spline`))
  (bind _returnvalue (* (`KismetMathLibrary.SelectInt` Index (+ Index 1) IsStart) (`self.MeshLength`)))
  (return (`SplineComponent.GetLocationAtDistanceAlongSpline` _spline _returnvalue "Local") (`KismetMathLibrary.ClampVectorSize` (`SplineComponent.GetTangentAtDistanceAlongSpline` _spline _returnvalue "Local") 0.0 (`self.MeshLength`))))

(fn `Setup Mat and RT`
  (bind _decal (`self.Decal`))
  (bind _materialref (`self.MaterialRef`))
  (bind (_decalsize_x _decalsize_y _decalsize_z) (`KismetMathLibrary.BreakVector` (`DecalComponent.DecalSize` (`self.Decal`))))
  (bind _returnvalue (`DecalComponent.CreateDynamicMaterialInstance` _decal))
  (bind _output_get (set `self.MaterialRef` _returnvalue))
  (`DecalComponent.SetDecalMaterial` _decal _output_get)
  (bind _returnvalue_2 (`KismetRenderingLibrary.CreateRenderTarget2D` (`KismetMathLibrary.FTrunc` _decalsize_y) (`KismetMathLibrary.FTrunc` _decalsize_z) "RTF_RG8"))
  (set `SceneCaptureComponent2D.TextureTarget` _returnvalue_2 (`self.SceneCaptureComponent2D`))
  (`MaterialInstanceDynamic.SetTextureParameterValue` _materialref "TextureToUse" _returnvalue_2)
  (`MaterialInstanceDynamic.SetVectorParameterValue` _materialref "BaseColor" (`self.Color`))
  (return))

(fn `Setup Mesh`
  (bind _output_get (set `self.MeshLength` (.x (`.BoxExtent` (`KismetMathLibrary.BreakBoxSphereBounds` (`StaticMesh.GetBounds` (defaults `Object` (`self.SplineMeshComponentClass`))))))))
  (bind _output_get_2 (set `self.SplineDivisions` (`KismetMathLibrary.FTrunc` (/ (`SplineComponent.GetSplineLength` (`self.Spline`)) _output_get))))
  (for _index (range (+ _output_get_2 1))
    (bind _returnvalue (`|AddComponentByClass` (`self.SplineMeshComponentClass`)))
    (`SplineMeshComponent.SetForwardAxis` _returnvalue "X" true)
    (bind (_position _tangent) (`self.CalculateSplineMeshStartEnd` _index true))
    (bind (_position_2 _tangent_2) (`self.CalculateSplineMeshStartEnd` _index))
    (`SplineMeshComponent.SetStartAndEnd` _returnvalue _position _tangent _position_2 _tangent_2 true)
    (`KismetArrayLibrary.Array_Add` (`self.SplineMeshes`) _returnvalue))
  (return))

(fn `UserConstructionScript`
  (bind _showonlyactors (`self.ShowOnlyActors`))
  (bind (_decalsize_x _decalsize_y _decalsize_z) (`KismetMathLibrary.BreakVector` (`DecalComponent.DecalSize` (`self.Decal`))))
  (`self.Setup Mat and RT`)
  (`self.ClearMeshes`
    (:`ExecOut`
      (`self.Setup Mesh`)
      (`KismetArrayLibrary.Array_Clear` _showonlyactors)
      (`KismetArrayLibrary.Array_Add` _showonlyactors self)
      (set `SceneCaptureComponent.ShowOnlyActors` _showonlyactors (`self.SceneCaptureComponent2D`))
      (set `SceneCaptureComponent2D.OrthoWidth` (* _decalsize_z 2.0) (`self.SceneCaptureComponent2D`)))))