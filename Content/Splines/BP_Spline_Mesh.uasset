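; Spline actor that projects its spline onto blocking geometry and lays spline meshes along the projected path.
; It samples the spline at intervals based on mesh length and projection resolution, line-tracing along the spline's default up vector.
; Hits form a second deformed spline, with one spline mesh component per segment and tangents clamped to mesh length.
; Construction and the CustomTick event clear and rebuild everything.
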(event `self.ReceiveBeginPlay`
  (`parent.ReceiveBeginPlay`)
  (set `self.MeshLength` (.x (`.BoxExtent` (`KismetMathLibrary.BreakBoxSphereBounds` (`StaticMesh.GetBounds` (defaults `Object` (`self.SplineMeshComponentClass`))))))))

(event `self.CustomTick`
  (`self.Clear Deformed Spline`)
  (bind _output_get (set `self.ResolutionLength` (/ (`self.MeshLength`) (`self.ProjectionResolution`))))
  (set `self.ResolutionDivisions` (`KismetMathLibrary.FTrunc` (/ (`SplineComponent.GetSplineLength` (`self.Spline`)) _output_get)))
  (`self.Cast and Add Points`)
  (`self.Mesh Deformed Spline`))

(fn `Cast and Add Points`
  (for _index (range (+ (`self.ResolutionDivisions`) 1))
    (bind _returnvalue (`SplineComponent.GetLocationAtDistanceAlongSpline` (`self.Spline`) (* _index (`self.ResolutionLength`)) "World"))
    (bind _outhit (`KismetSystemLibrary.LineTraceSingle` :`Start` _returnvalue :`End` (+ _returnvalue (* (`SplineComponent.GetDefaultUpVector` (`self.Spline`) "World") (`self.CastDistance`))) :`TraceChannel` "TraceTypeQuery1" :`DrawTime` 1.0))
    (bind (_bblockinghit _binitialoverlap _time _distance _location) (`GameplayStatics.BreakHitResult` _outhit))
    (if _bblockinghit
      (`SplineComponent.AddSplinePoint` (`self.DeformedSpline`) _location "World" true)))
  (return))

(fn `Clear Deformed Spline`
  (bind _splinemeshes (`self.SplineMeshes`))
  (for _array_element _splinemeshes
    (`ActorComponent.K2_DestroyComponent` _array_element))
  (`KismetArrayLibrary.Array_Clear` _splinemeshes)
  (`SplineComponent.ClearSplinePoints` (`self.DeformedSpline`) true)
  (return))

(fn `Mesh Deformed Spline`
  (bind _deformedspline (`self.DeformedSpline`))
  (bind _meshlength (`self.MeshLength`))
  (for _index (range (+ (- (`SplineComponent.GetNumberOfSplinePoints` (`self.DeformedSpline`)) 2) 1))
    (bind _returnvalue (`|AddComponentByClass` (`self.SplineMeshComponentClass`)))
    (`SplineMeshComponent.SetForwardAxis` _returnvalue "X" true)
    (bind (_location _tangent) (`SplineComponent.GetLocationAndTangentAtSplinePoint` _deformedspline _index "Local"))
    (bind (_location_2 _tangent_2) (`SplineComponent.GetLocationAndTangentAtSplinePoint` _deformedspline (+ _index 1) "Local"))
    (`SplineMeshComponent.SetStartAndEnd` _returnvalue _location (`KismetMathLibrary.ClampVectorSize` _tangent 0.0 _meshlength) _location_2 (`KismetMathLibrary.ClampVectorSize` _tangent_2 0.0 _meshlength) true)
    (`KismetArrayLibrary.Array_Add` (`self.SplineMeshes`) _returnvalue))
  (return))

(fn `UserConstructionScript`
  (`self.Clear Deformed Spline`)
  (bind _output_get (set `self.MeshLength` (.x (`.BoxExtent` (`KismetMathLibrary.BreakBoxSphereBounds` (`StaticMesh.GetBounds` (defaults `Object` (`self.SplineMeshComponentClass`))))))))
  (bind _output_get_2 (set `self.ResolutionLength` (/ _output_get (`self.ProjectionResolution`))))
  (set `self.ResolutionDivisions` (`KismetMathLibrary.FTrunc` (/ (`SplineComponent.GetSplineLength` (`self.Spline`)) _output_get_2)))
  (`self.Cast and Add Points`)
  (`self.Mesh Deformed Spline`))