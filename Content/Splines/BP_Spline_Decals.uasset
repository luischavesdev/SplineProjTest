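; Spline actor that lays a row of decal components along its spline path.
; The construction script divides spline length by DecalSize, then spawns decals at that spacing with a shared material and scale, each following the spline's yaw.
; Spawned decals are cached so each rebuild destroys the old set first.
; A CustomTick event repeats the full rebuild for play-mode spline edits and is optional for editor-only use.
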(event `self.ReceiveBeginPlay`
  (`parent.ReceiveBeginPlay`))

(event `self.CustomTick`
  ;[1 1 1] Can be discarded if spline is only to be edited while in editor and not in play mode
  (`self.Clear Decals`)
  (set `self.SplineDivisions` (`KismetMathLibrary.FTrunc` (/ (`SplineComponent.GetSplineLength` (`self.Spline`)) (`self.DecalSize`))))
  (`self.Spawn Decals`))

(fn `Clear Decals`
  (bind _decalscache (`self.DecalsCache`))
  (for _array_element _decalscache
    (`ActorComponent.K2_DestroyComponent` _array_element))
  (`KismetArrayLibrary.Array_Clear` _decalscache)
  (return))

(fn `Spawn Decals`
  (bind _spline (`self.Spline`))
  (for _index (range (+ (`self.SplineDivisions`) 1))
    (bind _returnvalue (`AddComponent|NODE_AddDecalComponent-1` :`RelativeTransform` (`KismetMathLibrary.MakeTransform` (0.0 0.0 0.0) (struct) (`self.DecalScale`))))
    (`DecalComponent.SetDecalMaterial` _returnvalue (`self.DecalMatRef`))
    (bind _returnvalue_2 (* _index (`self.DecalSize`)))
    (bind (_returnvalue_roll _returnvalue_pitch _returnvalue_yaw) (`KismetMathLibrary.BreakRotator` (`SplineComponent.GetRotationAtDistanceAlongSpline` _spline _returnvalue_2 "World")))
    (`SceneComponent.K2_SetWorldLocationAndRotation` _returnvalue (`SplineComponent.GetLocationAtDistanceAlongSpline` _spline _returnvalue_2 "World") (`KismetMathLibrary.MakeRotator` 0.0 0.0 _returnvalue_yaw) false false)
    (`KismetArrayLibrary.Array_Add` (`self.DecalsCache`) _returnvalue))
  (return))

(fn `UserConstructionScript`
  (`self.Clear Decals`)
  (set `self.SplineDivisions` (`KismetMathLibrary.FTrunc` (/ (`SplineComponent.GetSplineLength` (`self.Spline`)) (`self.DecalSize`))))
  (`self.Spawn Decals`))