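; Spline actor that projects its own shape as a colored line through a square decal.
; Construction and BeginPlay create a dynamic decal material and a render target sized to the decal, passed in as a texture parameter.
; DrawToRT samples the spline at even distances and draws canvas line segments from local XY into that target.
; Construction also draws, while CustomTick clears and redraws for play-mode spline edits.
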(event `self.ReceiveBeginPlay`
  (`parent.ReceiveBeginPlay`)
  (`self.Setup Mat and RT`))

(event `self.CustomTick`
  (bind (_decalsize_x _decalsize_y _decalsize_z) (`KismetMathLibrary.BreakVector` (`DecalComponent.DecalSize` (`self.Decal`))))
  ;[1 1 1] Can be discarded if spline is only to be edited while in editor and not in play mode
  (bind _output_get (set `self.DecalSize` _decalsize_z)) ; Assumes decal is always a square
  (set `self.DecalSizeHalf` (/ _output_get 2.0))
  (`KismetRenderingLibrary.ClearRenderTarget2D` (`self.RTRef`))
  (`self.Draw to RT`))

(fn `Draw to RT`
  (locals (SegmentLength :type "Float (double-precision)") (CanvasRef :type "Canvas Object Reference"))
  (bind _spline (`self.Spline`))
  (bind _segmentlength (`local.SegmentLength`))
  (set `local.SegmentLength` (/ (`SplineComponent.GetSplineLength` (`self.Spline`)) (`self.ProjectionResolution`)))
  (bind (_canvas _size _context) (`KismetRenderingLibrary.BeginDrawCanvasToRenderTarget` (`self.RTRef`)))
  (set `local.CanvasRef` _canvas)
  (for _index (range (`self.ProjectionResolution`))
    (bind (_returnvalue_x _returnvalue_y) (`KismetMathLibrary.BreakVector` (`SplineComponent.GetLocationAtDistanceAlongSpline` _spline (* _index _segmentlength) "Local")))
    (bind (_returnvalue_x_2 _returnvalue_y_2) (`KismetMathLibrary.BreakVector` (`SplineComponent.GetLocationAtDistanceAlongSpline` _spline (* _segmentlength (+ _index 1)) "Local")))
    (`Canvas.K2_DrawLine` (`local.CanvasRef`) (`self.PointInTextCoord` _returnvalue_x _returnvalue_y) (`self.PointInTextCoord` _returnvalue_x_2 _returnvalue_y_2) (`self.Thickness`) (struct :`R` 1.0 :`G` 1.0 :`B` 1.0 :`A` 1.0)))
  (`KismetRenderingLibrary.EndDrawCanvasToRenderTarget` _context)
  (return))

(fn `Setup Mat and RT`
  (bind _decal (`self.Decal`))
  (bind _materialref (`self.MaterialRef`))
  (bind _returnvalue (`KismetMathLibrary.FTrunc` (`self.DecalSize`)))
  (bind _returnvalue_2 (`DecalComponent.CreateDynamicMaterialInstance` _decal))
  (bind _output_get (set `self.MaterialRef` _returnvalue_2))
  (`DecalComponent.SetDecalMaterial` _decal _output_get)
  (bind _returnvalue_3 (`KismetRenderingLibrary.CreateRenderTarget2D` _returnvalue _returnvalue "RTF_RG8"))
  (bind _output_get_2 (set `self.RTRef` _returnvalue_3))
  (`MaterialInstanceDynamic.SetTextureParameterValue` _materialref "TextureToUse" _output_get_2)
  (`MaterialInstanceDynamic.SetVectorParameterValue` _materialref "BaseColor" (`self.Color`))
  (return))

(fn `UserConstructionScript`
  (bind (_decalsize_x _decalsize_y _decalsize_z) (`KismetMathLibrary.BreakVector` (`DecalComponent.DecalSize` (`self.Decal`))))
  (bind _output_get (set `self.DecalSize` _decalsize_z)) ; Assumes decal is always a square
  (set `self.DecalSizeHalf` (/ _output_get 2.0))
  (`self.Setup Mat and RT`)
  (`self.Draw to RT`))